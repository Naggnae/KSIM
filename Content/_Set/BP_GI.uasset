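; BP_GI, likely the GameInstance, builds BIM building levels and their topology graph from XML data.
; CreateBuildingOneFloor loads a level's mesh data through the XML parser subsystem, then has BPBIM create walls, floors, columns and objects and spawn doors.
; BPTopology then spawns nodes and draws the lines for that level.
; CreateBuildingAllFloor repeats this pipeline for every entry in LevelList.
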(fn CreateBuildingOneFloor
  (params (LevelName :type String))
  (bind _bp_bim (Variables|Default|GetBP_BIM))
  (bind _bp_topology (Variables|Default|GetBP_Topology))
  (Class|XMLParserSS|SetMeshDataList (Subsystems|GetXMLParserSS) LevelName)
  (Default|CreateWallMesh _bp_bim)
  (Default|CreateFloorMesh _bp_bim)
  (Default|CreateColumnMesh _bp_bim)
  (Default|CreateObjectMesh _bp_bim)
  (Default|SpawnDoor _bp_bim)
  (Default|SpawnNode _bp_topology)
  (Default|DrawTopologyLine _bp_topology)
  (return))

(fn CreateBuildingAllFloor
  (for _array_element (Variables|Default|GetLevelList)
    (CallFunction|CreateBuildingOneFloor _array_element))
  (return))