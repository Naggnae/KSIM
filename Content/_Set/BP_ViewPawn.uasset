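; BP_ViewPawn is a free-moving view camera pawn with rotate, pan and zoom controls.
; Holding the Rotation or Move action opens a gate on Tick, so axis input is applied every frame without delta-time scaling.
; Rotation adds pitch and yaw to the Camera, while Move pans the root along the camera's right and up vectors.
; Zoom dollies the root along the camera's forward vector rather than changing field of view.
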(event EventTick
  (params (DeltaSeconds :type Float%20%28single-precision%29))
  (Utilities|FlowControl|Sequence
    (:then_0
      (Utilities|FlowControl|Gate true
        (:Exit
          (CallFunction|Rotation))))
    (:then_1
      (Utilities|FlowControl|Gate true
        (:Exit
          (CallFunction|Move 2e+02))))))

(event Input|ActionEvents|InputActionRotation
  (params (Key :type Key%20Structure :default "None"))
  (:Pressed
    (Utilities|FlowControl|Gate true) ; enters at Open
  )
  (:Released
    (Utilities|FlowControl|Gate true) ; enters at Close
  ))

(event Input|ActionEvents|InputActionMove
  (params (Key :type Key%20Structure :default "None"))
  (:Pressed
    (Utilities|FlowControl|Gate true) ; enters at Open
  )
  (:Released
    (Utilities|FlowControl|Gate true) ; enters at Close
  ))

(event Input|AxisEvents|InputAxisZoom
  (params (AxisValue :type Float%20%28single-precision%29))
  (CallFunction|Zoom AxisValue 3e+02))

(fn ConstructionScript)

(fn Move
  (params (Distance :type Float%20%28single-precision%29))
  (bind _rootcomponent (Variables|Transformation|GetRootComponent))
  (bind _camera (Variables|Default|GetCamera))
  (Transformation|AddRelativeLocation _rootcomponent (* (Math|Vector|GetRightVector _camera) (* Distance -1.0 (Class|Actor|GetInputAxisKeyValue))) false false)
  (Transformation|AddRelativeLocation _rootcomponent (* (Math|Vector|GetUpVector _camera) (* Distance -1.0 (Class|Actor|GetInputAxisKeyValue))) false false))

(fn Zoom
  (params (Axis :type Float%20%28single-precision%29) (Distance :type Float%20%28single-precision%29))
  (Transformation|AddRelativeLocation (Variables|Transformation|GetRootComponent) (* (Math|Rotator|GetRotationXVector (Transformation|GetWorldRotation (Variables|Default|GetCamera))) (* Axis Distance)) false false))

(fn Rotation
  (Transformation|AddRelativeRotation (Variables|Default|GetCamera) (Math|Rotator|MakeRotator 0.0 (Class|Actor|GetInputAxisKeyValue) (Class|Actor|GetInputAxisKeyValue)) false false))