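; BIM building actor that rebuilds one or all levels at runtime from XML data parsed into BP_GI.
; OneFloor creates procedural meshes for walls, curtain walls, floors, columns and objects, triangulating floor polylines and grid-indexing columns, and caches structural components in the game instance.
; It also spawns doors and topology nodes, which DrawTopology links with spline meshes by target ID and InitTopology clears.
; Key 1 prints column components for debugging.
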(event EventBeginPlay
  (Variables|Default|SetGI (.AsBP%20GI (Utilities|Casting|CastToBP_GI (Game|GetGameInstance))))
  (Input|EnableInput (Game|GetPlayerController 0)))

(event Input|KeyboardEvents|1
  (params (Key :type Key%20Structure))
  (:Pressed
    (for _array_element (Variables|/Script/KSIM.GI|GetColumnMeshComponents (Variables|Default|GetGI))
      (Development|PrintString (Utilities|GetDisplayName _array_element)))))

(fn ConstructionScript)

(fn CreateMesh
  (params (Vertices :type Array%20of%20Vectors) (Triangles :type Array%20of%20Integers) (UV0 :type Array%20of%20Vector%202D%20Structures) (isCollision :type Boolean))
  (bind _returnvalue (AddComponent|AddProceduralMeshComponent true))
  (Class|ProceduralMeshComponent|CreateMeshSectionLinearColor _returnvalue 0 Vertices Triangles 0 UV0 0 0 0 0 0 isCollision)
  (return _returnvalue))

(fn OneFloor
  (params (LevelName :type String))
  (Class|XMLParserSS|SetMeshDataList (Subsystems|GetXMLParserSS) LevelName)
  (Utilities|FlowControl|Sequence
    (:then_0
      (for _array_element (Variables|/Script/KSIM.GI|GetWallMeshDataList (Variables|Default|GetGI))
        (bind _proceduralmesh (CallFunction|CreateMesh (.VertexList (Utilities|Struct|BreakWallMeshData _array_element)) (.TriangleIndexList (Utilities|Struct|BreakWallMeshData _array_element)) (Variables|Default|GetUV0) false))
        (switch string (.Type (Utilities|Struct|BreakWallMeshData _array_element))
          (:Wall
            (Utilities|Array|Add (Variables|/Script/KSIM.GI|GetWallMeshComponents (Variables|Default|GetGI)) _proceduralmesh)
            (Rendering|Material|SetMaterial _proceduralmesh 0 "/Game/Resources/StarterContent/Materials/M_Basic_Wall.M_Basic_Wall"))
          (:CurtainWall
            (Utilities|Array|Add (Variables|/Script/KSIM.GI|GetCurtainWallMeshComponents (Variables|Default|GetGI)) _proceduralmesh)
            (Rendering|Material|SetMaterial _proceduralmesh 0 "/Game/Material/M_Curtain.M_Curtain")))))
    (:then_1
      (for _array_element_2 (Variables|/Script/KSIM.GI|GetFloorMeshDataList (Variables|Default|GetGI))
        (bind _returnvalue (Class|TriangulatorBPLibrary|TriangulatorSampleFunction (Utilities|Array|MakeArray (Utilities|Struct|MakePolyline (.VertexList (Utilities|Struct|BreakFloorMeshData _array_element_2))))))
        (bind _output_get (Variables|Default|SetTriangle _returnvalue))
        (Utilities|Array|Reverse _output_get)
        (bind _proceduralmesh_2 (CallFunction|CreateMesh (.VertexList (Utilities|Struct|BreakFloorMeshData _array_element_2)) (Variables|Default|GetTriangle) (Variables|Default|GetUV0) false))
        (Utilities|Array|Add (Variables|/Script/KSIM.GI|GetFloorMeshComponents (Variables|Default|GetGI)) _proceduralmesh_2)
        (Rendering|Material|SetMaterial _proceduralmesh_2 0 "/Game/Material/M_Floor.M_Floor")))
    (:then_2
      (for _array_element_3 (Variables|/Script/KSIM.GI|GetColumnMeshDataList (Variables|Default|GetGI))
        (bind _triangles (CallFunction|SetColumnTriangle (.VertexList (Utilities|Struct|BreakColumnMeshData _array_element_3))))
        (bind _proceduralmesh_3 (CallFunction|CreateMesh (.VertexList (Utilities|Struct|BreakColumnMeshData _array_element_3)) _triangles (Variables|Default|GetUV0) false))
        (Utilities|Array|Add (Variables|/Script/KSIM.GI|GetColumnMeshComponents (Variables|Default|GetGI)) _proceduralmesh_3)
        (Rendering|Material|SetMaterial _proceduralmesh_3 0 "/Game/Resources/StarterContent/Materials/M_Basic_Wall.M_Basic_Wall")))
    (:then_3
      (for _array_element_4 (Variables|/Script/KSIM.GI|GetNodeDataList (Variables|Default|GetGI))
        (bind _returnvalue_2 (Game|SpawnActorfromClass "/Game/Actor/BP_Node.BP_Node_C" (Math|Transform|MakeTransform (.Location (Utilities|Struct|BreakNodeData _array_element_4)) "0, 0, 0" "1,1,1") "Undefined" 0 0))
        (Utilities|Array|Add (Variables|Default|GetNode) _returnvalue_2))
      (CallFunction|DrawTopology))
    (:then_4
      (for _array_element_5 (Variables|/Script/KSIM.GI|GetObjectMeshDataList (Variables|Default|GetGI))
        (CallFunction|CreateMesh (.VertexList (Utilities|Struct|Break3DObjectData _array_element_5)) (.TriangleIndexList (Utilities|Struct|Break3DObjectData _array_element_5)) (Variables|Default|GetUV0) false)))
    (:then_5
      (for _array_element_6 (Variables|/Script/KSIM.GI|GetDoorDataList (Variables|Default|GetGI))
        (Game|SpawnActorfromClass "/Game/Actor/BP_Door.BP_Door_C" (Math|Transform|MakeTransform (.Location (Utilities|Struct|BreakDoorData _array_element_6)) (.Direction (Utilities|Struct|BreakDoorData _array_element_6)) "1,1,1") "Undefined" 0 0)))))

(fn AllFloor
  (for _array_element (Variables|/Script/KSIM.GI|GetLevelList (Variables|Default|GetGI))
    (CallFunction|OneFloor _array_element)))

(fn DrawTopology
  (for _array_element (Variables|/Script/KSIM.GI|GetNodeDataList (Variables|Default|GetGI))
    (Utilities|Map|Add (Variables|Default|GetTopologyIDLocation) (.ID (Utilities|Struct|BreakNodeData _array_element)) (.Location (Utilities|Struct|BreakNodeData _array_element))))
  (for _array_element_2 (Variables|/Script/KSIM.GI|GetNodeDataList (Variables|Default|GetGI))
    (for _array_element_3 (.TargetIDs (Utilities|Struct|BreakNodeData _array_element_2))
      (bind _returnvalue (AddComponent|AddSplineMeshComponent true))
      (if (not (Math|Vector|Equal(Vector) (.Value (Utilities|Map|Find (Variables|Default|GetTopologyIDLocation) _array_element_3)) "0,0.000000, 0" 0.0001))
        (SplineMesh|SetStartandEnd _returnvalue (.Location (Utilities|Struct|BreakNodeData _array_element_2)) "0, 0, 0" (.Value (Utilities|Map|Find (Variables|Default|GetTopologyIDLocation) _array_element_3)) "0, 0, 0" true :!class /Script/Engine.SplineMeshComponent)
        (Utilities|Array|Add (Variables|Default|GetSplineMesh) _returnvalue)))))

(fn InitTopology
  (for _array_element (Variables|Default|GetSplineMesh)
    (Components|DestroyComponent _array_element))
  (for _array_element_2 (Variables|Default|GetNode)
    (Actor|DestroyActor _array_element_2))
  (Utilities|Array|Clear (Variables|Default|GetSplineMesh))
  (Utilities|Array|Clear (Variables|Default|GetNode)))

(fn SetColumnTriangle
  (params (Vertex :type Array%20of%20Vectors))
  (bind _triangles (Class|KismetProceduralMeshLibrary|CreateGridMeshTriangles (/ (Utilities|Array|Length Vertex) 2) 2 false))
  (return _triangles))